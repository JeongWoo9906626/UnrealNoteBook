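; AI controller for the MiddleJump monster that sets up its blackboard and runs the BT_AI_MiddleJump behavior tree.
; On BeginPlay it uses BB_AI, seeds MoveLocation and starts the tree.
; The patrol location is a random reachable point near the first BP_AITargetPoint found, queried through the NQF_MiddleJump navigation filter.
; Tick repeats that actor search and overwrites MoveLocation every frame.
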(event EventBeginPlay
  (bind _blackboardcomponent (Class|AIController|UseBlackboard "/Game/Monster/AI/BB_AI.BB_AI"))
  (Variables|Default|SetCurrentBlackBoard _blackboardcomponent)
  ;[1 1 1] Patrol 위치 정하기 (BP_AITargetPoint)
  (bind _outactors (Actor|GetAllActorsOfClass "/Game/Monster/BP_AITargetPoint.BP_AITargetPoint_C"))
  (AI|Components|Blackboard|SetValueasVector (Variables|Default|GetCurrentBlackBoard) (Utilities|Name|MakeLiteralName "MoveLocation") (.RandomLocation (AI|Navigation|GetRandomReachablePointinRadius (Transformation|GetActorLocation (Utilities|Array|Get(acopy) _outactors)) 25.0 0 "/Game/Monster/Navigation/NavigationQueryFilter/NQF_MiddleJump.NQF_MiddleJump_C")))
  (AI|RunBehaviorTree "/Game/Monster/AI/BT_AI_MiddleJump.BT_AI_MiddleJump"))

(event EventTick
  (params (DeltaSeconds :type Float%20%28single-precision%29))
  ;[1 1 1] Patrol 위치 정하기 (BP_AITargetPoint)
  (bind _outactors (Actor|GetAllActorsOfClass "/Game/Monster/BP_AITargetPoint.BP_AITargetPoint_C"))
  (AI|Components|Blackboard|SetValueasVector (Variables|Default|GetCurrentBlackBoard) (Utilities|Name|MakeLiteralName "MoveLocation") (.RandomLocation (AI|Navigation|GetRandomReachablePointinRadius (Transformation|GetActorLocation (Utilities|Array|Get(acopy) _outactors)) 25.0 0 "/Game/Monster/Navigation/NavigationQueryFilter/NQF_MiddleJump.NQF_MiddleJump_C"))))

(fn ConstructionScript)